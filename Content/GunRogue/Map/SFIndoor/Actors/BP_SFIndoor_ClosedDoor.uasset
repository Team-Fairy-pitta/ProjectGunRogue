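; Sliding door actor for the SFIndoor map that moves vertically when toggled through ActivateDoor.
; ActivateDoor calls Open or Close based on Isopen, and each sets the flag and plays its own timeline.
; The timelines lerp the door mesh's relative location up or down by Height from StartLocation.
; On finish, StartLocation is overwritten with a hard-coded X offset and Z of plus Height after opening, minus Height after closing.
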(event Custom|Open
  (Variables|Default|Setisopen? true)
  (bind _새_트랙_0 (Timeline|타임라인 PlayFromStart)
    (:Update
      (Transformation|SetRelativeLocation (Variables|Default|GetSM_Hall_Door_L1) (Math|Vector|Lerp(Vector) (Variables|Default|GetStartLocation) (+ (Variables|Default|GetStartLocation) (Math|Vector|MakeVector 0.0 0.0 (Variables|Default|GetHeight))) _새_트랙_0) false false))
    (:Finished
      (Variables|Default|SetStartLocation (Math|Vector|MakeVector -7.8e+02 0.0 (Variables|Default|GetHeight))))))

(event Custom|Close
  (Variables|Default|Setisopen? false)
  (bind _새_트랙_0 (Timeline|타임라인_0 PlayFromStart)
    (:Update
      (Transformation|SetRelativeLocation (Variables|Default|GetSM_Hall_Door_L1) (Math|Vector|Lerp(Vector) (Variables|Default|GetStartLocation) (- (Variables|Default|GetStartLocation) (Math|Vector|MakeVector 0.0 0.0 (Variables|Default|GetHeight))) _새_트랙_0) false false))
    (:Finished
      (Variables|Default|SetStartLocation (Math|Vector|MakeVector -7.8e+02 0.0 (* (Variables|Default|GetHeight) -1.0))))))

(event EventActivateDoor
  (if (Variables|Default|Getisopen?)
    (CallFunction|Close)
    (else
      (CallFunction|Open))))

(fn ConstructionScript)