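; Player character Blueprint that registers itself in BP_GRGameState's player list on BeginPlay.
; Its spectator events (next, previous, reset, view-target RPC) are empty, with their former logic left disconnected and never run.
; That unused logic cycles an index through the player list, wrapping past slot 0, skipping dead players and switching the view target with blend.
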(event Custom|ServerRPC_Spectator
  (params (타깃 :type Player%20Controller%20Object%20Reference) (NewViewTarget :type Actor%20Object%20Reference)))

(event EventBeginPlay
  (bind _asbp_grgame_state (Utilities|Casting|CastToBP_GRGameState (Game|GetGameState)))
  (bind _output_get (Variables|Default|SetGameState%20REF _asbp_grgame_state))
  (Default|AddPlayertoList _output_get self))

(event EventSpectateNextPlayer)

(event EventSpectatePreviousPlayer)

(event EventResetSpectatePlayer)

(fn ConstructionScript)