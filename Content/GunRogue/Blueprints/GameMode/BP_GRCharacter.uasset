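; BP_GRCharacter is a GunRogue player character with debug-key spectating of other players after death.
; On BeginPlay it adds itself to the BP_GRGameState player list.
; When dead, Up/Down cycle through that list, skipping index 0, while R returns to index 0 regardless of death state and 1 simulates death.
; View switches go through a spectator server RPC that calls SetViewTargetWithBlend on player controller 0.
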(event Custom|ServerRPC_Spectator
  (params (타깃 :type Player%20Controller%20Object%20Reference) (NewViewTarget :type Actor%20Object%20Reference))
  (Game|Player|SetViewTargetwithBlend 타깃 NewViewTarget 0.0 "VTBlend_Linear" 0.0 false))

(event EventBeginPlay
  (bind _asbp_grgame_state (Utilities|Casting|CastToBP_GRGameState (Game|GetGameState)))
  (bind _output_get (Variables|Default|SetGameState%20REF _asbp_grgame_state))
  (Default|AddPlayertoList _output_get self))

(event EventSpectateNextPlayer
  (bind _gamestate_ref (Variables|Default|GetGameState%20REF))
  (bind _playerlist (Variables|/Game/GunRogue/Blueprints/GameMode/BP_GRGameState.BP_GRGameState_C|GetPlayerList _gamestate_ref))
  (if (== (+ (Variables|Default|GetCurrentPlayer) 1) (Utilities|Array|Length _playerlist))
    (Variables|Default|SetCurrentPlayer 1)
    (else
      (Variables|Default|SetCurrentPlayer (+ (Variables|Default|GetCurrentPlayer) 1))))
  (CallFunction|ServerRPCSpectator (Game|GetPlayerController 0) (Utilities|Array|Get(acopy) _playerlist (Variables|Default|GetCurrentPlayer))))

(event EventSpectatePreviousPlayer
  (bind _gamestate_ref (Variables|Default|GetGameState%20REF))
  (bind _playerlist (Variables|/Game/GunRogue/Blueprints/GameMode/BP_GRGameState.BP_GRGameState_C|GetPlayerList _gamestate_ref))
  (if (== (- (Variables|Default|GetCurrentPlayer) 1) 0)
    (Variables|Default|SetCurrentPlayer (- (Utilities|Array|Length _playerlist) 1))
    (else
      (Variables|Default|SetCurrentPlayer (- (Variables|Default|GetCurrentPlayer) 1))))
  (CallFunction|ServerRPCSpectator (Game|GetPlayerController 0) (Utilities|Array|Get(acopy) _playerlist (Variables|Default|GetCurrentPlayer))))

(event EventResetSpectatePlayer
  (CallFunction|ServerRPCSpectator (Game|GetPlayerController 0) (Utilities|Array|Get(acopy) (Variables|/Game/GunRogue/Blueprints/GameMode/BP_GRGameState.BP_GRGameState_C|GetPlayerList (Variables|Default|GetGameState%20REF)))))

(event Input|KeyboardEvents|DebugKeyUp
  (params (Key :type Key%20Structure :default "None") (ActionValue :type Input%20Action%20Value%20Structure))
  (:Pressed
    (if (Variables|Default|Getisdead?)
      (Class|GRCharacter|CallSpectateNextPlayer))))

(event Input|KeyboardEvents|DebugKeyDown
  (params (Key :type Key%20Structure :default "None") (ActionValue :type Input%20Action%20Value%20Structure))
  (:Pressed
    (if (Variables|Default|Getisdead?)
      (Class|GRCharacter|CallSpectatePreviousPlayer))))

(event Input|KeyboardEvents|DebugKey1
  (params (Key :type Key%20Structure :default "None") (ActionValue :type Input%20Action%20Value%20Structure))
  (:Pressed
    (Variables|Default|Setisdead? true)
    (Development|PrintString "죽음상태!" true true "(R=0.000000,G=0.660000,B=1.000000,A=1.000000)" 5.0)))

(event Input|KeyboardEvents|DebugKeyR
  (params (Key :type Key%20Structure :default "None") (ActionValue :type Input%20Action%20Value%20Structure))
  (:Pressed
    (Class|GRCharacter|CallResetSpectatePlayer)))

(fn ConstructionScript)