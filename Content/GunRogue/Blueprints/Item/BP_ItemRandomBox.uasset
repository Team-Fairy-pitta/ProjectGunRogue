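; BP_ItemRandomBox is a random item box that plays a lid-opening animation for the player who opens it.
; StartOpenAnimation tilts the lid's world pitch with a Timeline only when the given GRPlayerState belongs to player controller ID 0.
; Regardless of that check, the authority waits a fixed delay meant to match the animation length, then calls OnFinishOpenAnimation with that player state.
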(event EventStartOpenAnimation
  (params (GRPlayerState :type GR%20Player%20State%20Object%20Reference))
  (if (== GRPlayerState (Variables|/Script/Engine.Controller|GetPlayerState (Class|GameplayStatics|GetPlayerControllerfromID)))
    (Utilities|FlowControl|Sequence
      (:then_0
        (bind _newtrack_0 (Timeline|Timeline Play)
          (:Update
            (Transformation|SetWorldRotation (Variables|Default|GetBoxLid) (Math|Rotator|MakeRotator 0.0 (* -5e+01 _newtrack_0) 0.0) false false))))
      (:then_1
        (Networking|SwitchHasAuthority :!label _label
          (:Authority
            ;[0.15 0.15 0.15 0.5] Duration: 뚜껑 애니메이션 시간
            (Utilities|FlowControl|Delay 1.0)
            (Class|GRItemRandomBox|OnFinishOpenAnimation GRPlayerState)))))
    (else
      (goto _label))))

(fn ConstructionScript)