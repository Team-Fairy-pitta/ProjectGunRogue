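; BP_Door is a door in the GunRogue level streaming folder that slides its mesh vertically to open and close.
; ActivateDoor checks Isopen and calls Open or Close, which set the flag and play separate timelines.
; Each timeline lerps DoorMesh's relative location 300 units up or down from StartLocation.
; On finish, StartLocation is overwritten with a fixed +300 or -300 Z vector, not the mesh's actual end position.
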(event Custom|Open
  (Variables|Default|Setisopen? true)
  (bind _새_트랙_0 (Timeline|OpenDoor PlayFromStart)
    (:Update
      (Transformation|SetRelativeLocation (Variables|Default|GetDoorMesh) (Math|Vector|Lerp(Vector) (Variables|Default|GetStartLocation) (+ (Variables|Default|GetStartLocation) "0.000000,0.000000,300.000000") _새_트랙_0) false false))
    (:Finished
      (Variables|Default|SetStartLocation "0.000000,0.000000,300.000000"))))

(event Custom|Close
  (Variables|Default|Setisopen? false)
  (bind _새_트랙_0 (Timeline|CloseDoor PlayFromStart)
    (:Update
      (Transformation|SetRelativeLocation (Variables|Default|GetDoorMesh) (Math|Vector|Lerp(Vector) (Variables|Default|GetStartLocation) (- (Variables|Default|GetStartLocation) "0.000000,0.000000,300.000000") _새_트랙_0) false false))
    (:Finished
      (Variables|Default|SetStartLocation "0.000000,0.000000,-300.000000"))))

(event EventActivateDoor
  (if (Variables|Default|Getisopen?)
    (CallFunction|Close)
    (else
      (CallFunction|Open))))

(fn ConstructionScript)